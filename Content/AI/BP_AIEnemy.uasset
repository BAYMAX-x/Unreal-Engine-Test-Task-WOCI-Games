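; BP_AIEnemy is a melee AI enemy that fights the player and shows a proximity-based health bar.
; Its Attack event sphere-traces pawns around itself, damages the given target and plays a werewolf attack montage.
; Overlap with a punching player reduces Health, updates the widget and plays impact feedback; at zero it plays a random death montage and destroys itself.
; A Sphere component toggles health widget visibility as the player enters or leaves.
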(event `/Game/AI/BPI_Enemy.Attack`
  (params (TargetActor :type "Actor Object Reference"))
  (bind _returnvalue (`self.K2_GetActorLocation`))
  ; Comment
  (bind (_outhits _returnvalue_2) (`KismetSystemLibrary.SphereTraceMultiForObjects` _returnvalue _returnvalue 200.0 (`|MakeArray` "ObjectTypeQuery3" :!type "EObjectTypeQuery Enum")))
  (if _returnvalue_2
    (for _array_element _outhits
      (bind (_bblockinghit _binitialoverlap _time _distance _location _impactpoint _normal _impactnormal _physmat _hitactor) (`GameplayStatics.BreakHitResult` _array_element))
      (if (== TargetActor _hitactor)
        (`GameplayStatics.ApplyDamage` _hitactor 10.0)
        (`|PlayMontage` (`self.Mesh`) "/Game/Werewolf/Animations/Anim_Werewolf_attack1_Montage.Anim_Werewolf_attack1_Montage"
          (:`then`
            (break)))))))

(event `self.ReceiveActorBeginOverlap`
  (params (OtherActor :type "Actor Object Reference"))
  ; animation
  (bind _asbp_gameplay_player (cast `/Game/TFPMovement/Player/Blueprint/BP_GameplayPlayer` OtherActor))
  (if (`/Game/TFPMovement/Player/Blueprint/BP_GameplayPlayer.IsPunching` _asbp_gameplay_player)
    (`GameplayStatics.PlaySoundAtLocation` "/Game/Sound/Punch/punch_Cue.punch_Cue" (`self.K2_GetActorLocation`) (struct) 1.0 1.0 0.0 null null null null)
    (bind _returnvalue (`self.PlayAnimMontage` "/Game/Animation/Animations/Impact_mixamo_com_Montage.Impact_mixamo_com_Montage"))
    (bind _output_get (set `self.Health` (- (`self.Health`) (`self.Damage`))))
    (set `/Game/Health/AI_Health/AI_Health_HUD.Health` (`KismetMathLibrary.Conv_IntToDouble` _output_get) (`self.HealthWidgetRef`))
    (`KismetSystemLibrary.Delay` _returnvalue)
    (if (<= _output_get 0)
      (`GameplayStatics.PlaySoundAtLocation` "/Game/Sound/Death/Death_Cue.Death_Cue" (`self.K2_GetActorLocation`) (struct) 1.0 1.0 0.0 null null null null)
      (bind _returnvalue_2 (`self.PlayAnimMontage` (`|GetArrayItem` (`self.Dying Montage Array`) (`KismetMathLibrary.RandomIntegerInRange` 0 2))))
      (`KismetSystemLibrary.Delay` (- _returnvalue_2 0.5))
      (`self.K2_DestroyActor`))))

(event `self.ReceiveBeginPlay`
  (bind _asai_health_hud (cast `/Game/Health/AI_Health/AI_Health_HUD` (`WidgetComponent.GetUserWidgetObject` (`self.Health_Widget`))))
  (set `self.HealthWidgetRef` _asai_health_hud))

(event `self.Sphere.OnComponentBeginOverlap`
  (params (OverlappedComponent :type "PrimitiveComponent Object Reference") (OtherActor :type "Actor Object Reference") (OtherComp :type "PrimitiveComponent Object Reference") (OtherBodyIndex :type Integer) (bFromSweep :type Boolean) (SweepResult :type "HitResult Structure (by ref)"))
  ; Comment
  (cast `/Game/TFPMovement/Player/Blueprint/BP_GameplayPlayer` OtherActor)
  (`SceneComponent.SetVisibility` (`self.Health_Widget`) true false))

(event `self.Sphere.OnComponentEndOverlap`
  (params (OverlappedComponent :type "PrimitiveComponent Object Reference") (OtherActor :type "Actor Object Reference") (OtherComp :type "PrimitiveComponent Object Reference") (OtherBodyIndex :type Integer))
  ; Comment
  (cast `/Game/TFPMovement/Player/Blueprint/BP_GameplayPlayer` OtherActor)
  (`SceneComponent.SetVisibility` (`self.Health_Widget`) false false))

(fn `UserConstructionScript`)